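; BP_Player is the player character Blueprint, handling basic movement, look and jump through Enhanced Input.
; On BeginPlay it adds the IMC_PlayerInput mapping context to the first player's input subsystem.
; Move input drives movement along right and forward vectors built from control rotation with pitch zeroed, so looking up or down does not affect direction.
; Look input feeds controller yaw and pitch, and Jump fires when its action starts.
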(event `self.ReceiveBeginPlay`
  (`EnhancedInputSubsystemInterface.AddMappingContext` (pcsubsystem `EnhancedInputLocalPlayerSubsystem` (`GameplayStatics.GetPlayerController` 0)) "/Game/Input/IMC_PlayerInput.IMC_PlayerInput" 0 (struct)))

(event `EnhancedInput|/Game/Input/IA_Move`
  (params (ActionValue :type "Vector2D Structure") (ElapsedSeconds :type "Float (double-precision)") (TriggeredSeconds :type "Float (double-precision)") (InputAction :type "InputAction Object Reference" :default "/Game/Input/IA_Move.IA_Move"))
  (bind (_returnvalue_roll _returnvalue_pitch _returnvalue_yaw) (`KismetMathLibrary.BreakRotator` (`self.GetControlRotation`)))
  (bind (_returnvalue_roll_2 _returnvalue_pitch_2 _returnvalue_yaw_2) (`KismetMathLibrary.BreakRotator` (`self.GetControlRotation`)))
  (:`Triggered`
    (`self.AddMovementInput` (`KismetMathLibrary.GetRightVector` (`KismetMathLibrary.MakeRotator` _returnvalue_roll_2 0.0 _returnvalue_yaw_2)) ActionValue_X)
    (`self.AddMovementInput` (`KismetMathLibrary.GetForwardVector` (`KismetMathLibrary.MakeRotator` _returnvalue_roll 0.0 _returnvalue_yaw)) ActionValue_Y)))

(event `EnhancedInput|/Game/Input/IA_Look`
  (params (ActionValue :type "Vector2D Structure") (ElapsedSeconds :type "Float (double-precision)") (TriggeredSeconds :type "Float (double-precision)") (InputAction :type "InputAction Object Reference" :default "/Game/Input/IA_Look.IA_Look"))
  (:`Triggered`
    (`self.AddControllerYawInput` ActionValue_X)
    (bind _result (`/Engine/EditorBlueprintResources/StandardMacros.NegateFloat` ActionValue_Y)
      (:`  `
        (`self.AddControllerPitchInput` _result)))))

(event `EnhancedInput|/Game/Input/IA_Jump`
  (params (ActionValue :type Boolean) (ElapsedSeconds :type "Float (double-precision)") (TriggeredSeconds :type "Float (double-precision)") (InputAction :type "InputAction Object Reference" :default "/Game/Input/IA_Jump.IA_Jump"))
  (:`Started`
    (`self.Jump`)))

(fn `UserConstructionScript`)